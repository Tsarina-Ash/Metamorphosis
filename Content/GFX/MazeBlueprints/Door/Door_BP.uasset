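; Maze door Blueprint that slides open when the first-person character enters its Radius trigger and closes when they leave.
; Locked doors open only if the character's KeyRing contains the required key; otherwise a message is printed.
; A timeline lerps the Cube mesh downward from its starting relative location and plays in reverse to close it.
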(event `self.ReceiveBeginPlay`
  (set `self.Start Postition ` (`SceneComponent.RelativeLocation` (`self.Cube`))))

(event `OpenDoor`
  (bind _start_postition_ (`self.Start Postition `))
  (bind (_direction _speed) (`Timeline|Positition` :!label _label)
    (:`Update`
      (`SceneComponent.K2_SetRelativeLocation` (`self.Cube`) (`KismetMathLibrary.VLerp` _start_postition_ (- _start_postition_ (0.0 0.0 225.0)) _speed) false false))))

(event `CloseDoor`
  (goto _label :!via `Reverse`))

(event `self.Radius.OnComponentBeginOverlap`
  (params (OverlappedComponent :type "PrimitiveComponent Object Reference") (OtherActor :type "Actor Object Reference") (OtherComp :type "PrimitiveComponent Object Reference") (OtherBodyIndex :type Integer) (bFromSweep :type Boolean) (SweepResult :type "HitResult Structure (by ref)"))
  ;[1 0 0.02529] Open_Door
  (bind _asbp_first_person_character (cast `/Game/Player/FirstPerson/Blueprints/BP_FirstPersonCharacter` OtherActor))
  (if (`self.Locked?`)
    (if (`KismetArrayLibrary.Array_Contains` (`/Game/Player/FirstPerson/Blueprints/BP_FirstPersonCharacter.KeyRing` _asbp_first_person_character) (`self.KeyNeeded`))
      (`self.OpenDoor`)
      (set `self.DoorOpen?` true)
      (else
        (`KismetSystemLibrary.PrintString` "Unlock one of those doors!!!")))
    (else
      (`self.OpenDoor`)
      (set `self.DoorOpen?` true))))

(event `self.Radius.OnComponentEndOverlap`
  (params (OverlappedComponent :type "PrimitiveComponent Object Reference") (OtherActor :type "Actor Object Reference") (OtherComp :type "PrimitiveComponent Object Reference") (OtherBodyIndex :type Integer))
  ;[0 1 0.9795] Close_Door
  (cast `/Game/Player/FirstPerson/Blueprints/BP_FirstPersonCharacter` OtherActor)
  (if (`self.DoorOpen?`)
    (`self.CloseDoor`)
    (set `self.DoorOpen?` false)))

(fn `UserConstructionScript`)
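; KeyCard_BP is a keycard pickup in the maze's door assets.
; Overlapping its Radius component with the first-person character adds KeyID to that character's KeyRing without duplicates, then destroys the card.
; The construction script applies KeyMat to the cube and Lightcolor to its light, so each placed card can show its own look.
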(event `self.Radius.OnComponentBeginOverlap`
  (params (OverlappedComponent :type "PrimitiveComponent Object Reference") (OtherActor :type "Actor Object Reference") (OtherComp :type "PrimitiveComponent Object Reference") (OtherBodyIndex :type Integer) (bFromSweep :type Boolean) (SweepResult :type "HitResult Structure (by ref)"))
  (bind _asbp_first_person_character (cast `/Game/Player/FirstPerson/Blueprints/BP_FirstPersonCharacter` OtherActor))
  (`KismetArrayLibrary.Array_AddUnique` (`/Game/Player/FirstPerson/Blueprints/BP_FirstPersonCharacter.KeyRing` _asbp_first_person_character) (`self.KeyID`))
  (`self.K2_DestroyActor`))

(fn `UserConstructionScript`
  (`PrimitiveComponent.SetMaterial` (`self.Cube`) 0 (`self.KeyMat`))
  (`LightComponent.SetLightColor` (`self.Light`) (`self.Lightcolor`) true))